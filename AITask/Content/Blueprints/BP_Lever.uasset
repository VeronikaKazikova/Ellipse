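; Lever actor that players can interact with when nearby, built on the Gameplay Ability System.
; On BeginPlay it grants its own ability system the lever self-activation ability.
; Box overlap applies a ready-to-cast effect to the player, hands it a lever reference and notifies the GameMode.
; Leaving removes effects granting State.ReadyForLever, clears the reference and notifies the GameMode.
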(event `self.ReceiveBeginPlay`
  ;[0.5033 1 0.287] Begin Play
  (`AbilitySystemComponent.K2_GiveAbility` (`self.AbilitySystem`) "/Game/Blueprints/GAS_Abilities/GA_LeverActivateItself.GA_LeverActivateItself_C" 0 -1))

(event `self.Box.OnComponentBeginOverlap`
  (params (OverlappedComponent :type "PrimitiveComponent Object Reference") (OtherActor :type "Actor Object Reference") (OtherComp :type "PrimitiveComponent Object Reference") (OtherBodyIndex :type Integer) (bFromSweep :type Boolean) (SweepResult :type "HitResult Structure (by ref)"))
  ;[1 1 1] When a player is close to lever - make them know they can interact with it, store ref to this object in player class and let gamemode know it
  (bind _asbp_player_character (cast `/Game/Blueprints/Player/BP_PlayerCharacter` OtherActor))
  (`AbilitySystemComponent.BP_ApplyGameplayEffectToSelf` :`self` (`PlayerCharacter.AbilitySystemComponent` _asbp_player_character) :`GameplayEffectClass` "/Game/Blueprints/GameplayEffects/GE_ReadyToCast.GE_ReadyToCast_C")
  (`/Game/Blueprints/Player/BP_PlayerCharacter.StoreRefToLever` _asbp_player_character self)
  (`/Game/Blueprints/BP_GameMode.PlayerInLever` (cast `/Game/Blueprints/BP_GameMode` (`GameplayStatics.GetGameMode`) :!pure true)))

(event `self.Box.OnComponentEndOverlap`
  (params (OverlappedComponent :type "PrimitiveComponent Object Reference") (OtherActor :type "Actor Object Reference") (OtherComp :type "PrimitiveComponent Object Reference") (OtherBodyIndex :type Integer))
  ;[1 1 1] When player leaves proximity of lever, unable its activation option, erase reference to it and let gamemode know
  (bind _asbp_player_character (cast `/Game/Blueprints/Player/BP_PlayerCharacter` OtherActor))
  (`AbilitySystemComponent.RemoveActiveEffectsWithGrantedTags` (`PlayerCharacter.AbilitySystemComponent` _asbp_player_character) (struct :`GameplayTags` (struct :`(TagName` "State.ReadyForLever"))))
  (`/Game/Blueprints/Player/BP_PlayerCharacter.EraseRefToLever` _asbp_player_character)
  (`/Game/Blueprints/BP_GameMode.PlayerLeftLever` (cast `/Game/Blueprints/BP_GameMode` (`GameplayStatics.GetGameMode`) :!pure true)))

(fn `UserConstructionScript`)