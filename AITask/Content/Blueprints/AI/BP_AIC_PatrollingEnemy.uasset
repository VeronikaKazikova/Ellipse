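; AI controller for the patrolling enemy that runs the BT_PatrolAI behavior tree on possession.
; It forwards target perception updates, with actor and stimulus, to its controlled BP_AIPatrolEnemy pawn, which handles the response.
; Helper functions write the target actor, line-of-sight and player invisibility values to the Blackboard.
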(event `self.ReceivePossess`
  (params (PossessedPawn :type "Pawn Object Reference"))
  (`self.RunBehaviorTree` "/Game/Blueprints/AI/BT_PatrolAI.BT_PatrolAI"))

(event `self.AIPerceptionComponent.OnTargetPerceptionUpdated`
  (params (Actor :type "Actor Object Reference") (Stimulus :type "AIStimulus Structure"))
  ;[1 1 1] let patrol AI enemy know sight perception has been updated
  (bind _asbp_aipatrol_enemy (cast `/Game/Blueprints/AI/BP_AIPatrolEnemy` (`self.K2_GetPawn`)))
  (`/Game/Blueprints/AI/BP_AIPatrolEnemy.ControllerOnTargetPerceptionUpdated` _asbp_aipatrol_enemy Actor Stimulus))

(fn `UpdateHasLineOfSightKey`
  (params (HasLineOfSight :type Boolean))
  (`BlackboardComponent.SetValueAsBool` (`self.Blackboard`) (`self.HasLineOfSightName`) HasLineOfSight))

(fn `UpdateIsPlayerInvisibleKey`
  (params (IsPlayerInvisible :type Boolean))
  (`BlackboardComponent.SetValueAsBool` (`self.Blackboard`) (`self.IsPlayerInvisible`) IsPlayerInvisible))

(fn `UpdateTargetActorKey`
  (params (TargetActor :type "Actor Object Reference"))
  (`BlackboardComponent.SetValueAsObject` (`self.Blackboard`) (`self.TargetActorName`) TargetActor))

(fn `UserConstructionScript`)