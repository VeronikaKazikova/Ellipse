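; Patrolling enemy AI that relays what it perceives and the player's concealment state to its AI controller's Blackboard.
; On BeginPlay it binds to player dispatchers for bush and shapeshift changes, both driving one IsPlayerInvisible key.
; Either exit event clears that key without checking the other state.
; Perception updates set the target actor and line-of-sight keys when sensing succeeds and clear them otherwise.
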(event `self.ReceiveBeginPlay`
  ;[0.4742 1 0.5065] Begin play - save references and bind to dispatchers
  (set `self.PlayerRef` (cast `/Game/Blueprints/Player/BP_PlayerCharacter` (`GameplayStatics.GetPlayerPawn` 0) :!pure true))
  (set `self.AIControllerRef` (cast `/Game/Blueprints/AI/BP_AIC_PatrollingEnemy` (`self.GetController`) :!pure true))
  (add `/Game/Blueprints/Player/BP_PlayerCharacter.PlayerEntersBush` (`self.PlayerRef`) (delegate `PlayerIsInBush`))
  (add `/Game/Blueprints/Player/BP_PlayerCharacter.PlayerLeavesBush` (`self.PlayerRef`) (delegate `PlayerNotInBush`))
  (add `/Game/Blueprints/Player/BP_PlayerCharacter.PlayerShapeshifted` (`self.PlayerRef`) (delegate `PlayerInShapeshift`))
  (add `/Game/Blueprints/Player/BP_PlayerCharacter.PlayerInNormalnForm` (`self.PlayerRef`) (delegate `PlayerInNormalForm`)))

(event `PlayerInNormalForm`
  ;[0.4742 1 0.5065] Begin play - save references and bind to dispatchers
  (`/Game/Blueprints/AI/BP_AIC_PatrollingEnemy.UpdateIsPlayerInvisibleKey` (`self.AIControllerRef`) false))

(event `PlayerInShapeshift`
  ;[0.4742 1 0.5065] Begin play - save references and bind to dispatchers
  (`/Game/Blueprints/AI/BP_AIC_PatrollingEnemy.UpdateIsPlayerInvisibleKey` (`self.AIControllerRef`) true))

(event `PlayerNotInBush`
  ;[0.4742 1 0.5065] Begin play - save references and bind to dispatchers
  (`/Game/Blueprints/AI/BP_AIC_PatrollingEnemy.UpdateIsPlayerInvisibleKey` (`self.AIControllerRef`) false))

(event `PlayerIsInBush`
  ;[0.4742 1 0.5065] Begin play - save references and bind to dispatchers
  (`/Game/Blueprints/AI/BP_AIC_PatrollingEnemy.UpdateIsPlayerInvisibleKey` (`self.AIControllerRef`) true))

(event `ControllerOnTargetPerceptionUpdated`
  (params (PerceivedActor :type "Actor Object Reference") (PerceivedStimulus :type "AIStimulus Structure"))
  ;[1 1 1] On update Perception - either set target actor for AI in Blackboard or erase it if it is no longer perceived
  (set `self.PerceivedActor` PerceivedActor)
  (if (`.bSuccessfullySensed` (break `AIStimulus` PerceivedStimulus))
    (`/Game/Blueprints/AI/BP_AIC_PatrollingEnemy.UpdateTargetActorKey` (`self.AIControllerRef`) (`self.PerceivedActor`)) ; setting target actor in BB to perceived actor
    (`/Game/Blueprints/AI/BP_AIC_PatrollingEnemy.UpdateHasLineOfSightKey` (`self.AIControllerRef`) true) ; updating BB key to say there is active LOS
    (else
      (set `self.PerceivedActor` null) ; Null the ref for sensed target
      (`/Game/Blueprints/AI/BP_AIC_PatrollingEnemy.UpdateTargetActorKey` (`self.AIControllerRef`) null) ; nullifying Target Actor in BB
      (`/Game/Blueprints/AI/BP_AIC_PatrollingEnemy.UpdateHasLineOfSightKey` (`self.AIControllerRef`) false) ; updating BB key to say there is no current LOS
    )))

(fn `UserConstructionScript`)