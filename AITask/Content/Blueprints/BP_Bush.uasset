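; BP_Bush is a bush that hides characters standing inside it by making them invisible through the Gameplay Ability System.
; Box overlap begin applies GE_MakeInvisible to any actor with a valid ability system component, and overlap end removes active effects granting the Status.Invisible tag.
; For BP_PlayerCharacter actors, it also calls the player's enters-bush and leaves-bush calls on each transition.
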(event `self.Box.OnComponentBeginOverlap`
  (params (OverlappedComponent :type "PrimitiveComponent Object Reference") (OtherActor :type "Actor Object Reference") (OtherComp :type "PrimitiveComponent Object Reference") (OtherBodyIndex :type Integer) (bFromSweep :type Boolean) (SweepResult :type "HitResult Structure (by ref)"))
  (bind _returnvalue (`AbilitySystemBlueprintLibrary.GetAbilitySystemComponent` OtherActor))
  ;[1 1 1] Apply invisibility effect to player when overlapping with bush
  (`/Engine/EditorBlueprintResources/StandardMacros.IsValid` _returnvalue
    (:`Is Valid`
      (`AbilitySystemComponent.BP_ApplyGameplayEffectToTarget` :`self` _returnvalue :`GameplayEffectClass` "/Game/Blueprints/GameplayEffects/GE_MakeInvisible.GE_MakeInvisible_C" :`Target` _returnvalue)
      (bind _asbp_player_character (cast `/Game/Blueprints/Player/BP_PlayerCharacter` OtherActor))
      (`/Game/Blueprints/Player/BP_PlayerCharacter.PlayerEntersBush` _asbp_player_character))))

(event `self.Box.OnComponentEndOverlap`
  (params (OverlappedComponent :type "PrimitiveComponent Object Reference") (OtherActor :type "Actor Object Reference") (OtherComp :type "PrimitiveComponent Object Reference") (OtherBodyIndex :type Integer))
  (bind _returnvalue (`AbilitySystemBlueprintLibrary.GetAbilitySystemComponent` OtherActor))
  ;[1 1 1] Remove Invisibility Effect When Player Leaves Bush Collision Box
  (`/Engine/EditorBlueprintResources/StandardMacros.IsValid` _returnvalue
    (:`Is Valid`
      (`AbilitySystemComponent.RemoveActiveEffectsWithGrantedTags` _returnvalue (struct :`GameplayTags` (struct :`(TagName` "Status.Invisible"))))
      (bind _asbp_player_character (cast `/Game/Blueprints/Player/BP_PlayerCharacter` OtherActor))
      (`/Game/Blueprints/Player/BP_PlayerCharacter.PlayerLeavesBush` _asbp_player_character))))

(fn `UserConstructionScript`)