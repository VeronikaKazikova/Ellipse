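; Witch player character built on the Gameplay Ability System, handling jumping, shapeshifting, portals, levers, pausing and death.
; BeginPlay grants abilities and starting effects; input triggers abilities by tag, with lever use also activating the lever's own ability.
; Tick reports death to the game mode and toggles the grounded effect through DoOnce gates.
; Enemy overlaps add or remove damage effects; shapeshifting swaps meshes and disables input until a timer restores both.
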(event `self.ReceiveBeginPlay`
  (bind _abilitysystemcomponent (`self.AbilitySystemComponent`))
  ;[0.2633 1 0.4615] Begin play - learn ability system all abilities and apply initial effects
  (`AbilitySystemComponent.K2_GiveAbility` _abilitysystemcomponent "/Game/Blueprints/GAS_Abilities/GA_EnterPortal.GA_EnterPortal_C" 0 -1)
  (`AbilitySystemComponent.K2_GiveAbility` _abilitysystemcomponent "/Game/Blueprints/GAS_Abilities/GA_UnlockLever.GA_UnlockLever_C" 0 -1)
  (`AbilitySystemComponent.K2_GiveAbility` _abilitysystemcomponent "/Game/Blueprints/GAS_Abilities/GA_Shapeshift.GA_Shapeshift_C" 0 -1)
  (`AbilitySystemComponent.K2_GiveAbility` _abilitysystemcomponent "/Game/Blueprints/GAS_Abilities/GA_Jump.GA_Jump_C" 0 -1)
  (`AbilitySystemComponent.BP_ApplyGameplayEffectToSelf` :`self` (`self.AbilitySystemComponent`) :`GameplayEffectClass` "/Game/Blueprints/GameplayEffects/GE_WitchInit.GE_WitchInit_C")
  (`self.CheckGrounded`)
  (`AbilitySystemComponent.BP_ApplyGameplayEffectToSelf` :`self` (`self.AbilitySystemComponent`) :`GameplayEffectClass` "/Game/Blueprints/GameplayEffects/GE_RegenerateMana.GE_RegenerateMana_C"))

(event `self.ReceiveTick`
  (params (DeltaSeconds :type "Float (single-precision)"))
  ;[1 0.3737 0.3538] Tick
  (`self.CheckGrounded`)
  (`self.CheckIfDead`))

(event `OnFalling`
  ;[1 1 1] Add/remove grounded tag as player jumps
  (`/Engine/EditorBlueprintResources/StandardMacros.DoOnce` false :!label _label
    (:`Completed`
      (`AbilitySystemComponent.RemoveActiveEffectsWithGrantedTags` (`self.AbilitySystemComponent`) (struct :`GameplayTags` (struct :`(TagName` "Status.Grounded"))))
      (goto _label_2 :!via `Reset`))))

(event `OnGrounded`
  ;[1 1 1] Add/remove grounded tag as player jumps
  (`/Engine/EditorBlueprintResources/StandardMacros.DoOnce` false :!label _label_2
    (:`Completed`
      (`AbilitySystemComponent.BP_ApplyGameplayEffectToSelf` :`self` (`self.AbilitySystemComponent`) :`GameplayEffectClass` "/Game/Blueprints/GameplayEffects/GE_SetGrounded.GE_SetGrounded_C")
      (goto _label :!via `Reset`))))

(event `self.HitBox.OnComponentBeginOverlap`
  (params (OverlappedComponent :type "PrimitiveComponent Object Reference") (OtherActor :type "Actor Object Reference") (OtherComp :type "PrimitiveComponent Object Reference") (OtherBodyIndex :type Integer) (bFromSweep :type Boolean) (SweepResult :type "HitResult Structure (by ref)"))
  ;[1 1 1] If enemy is in range, apply take damage tag to itself
  (cast `/Game/Blueprints/AI/BP_AIPatrolEnemy` OtherActor)
  (`AbilitySystemComponent.BP_ApplyGameplayEffectToSelf` :`self` (`self.AbilitySystemComponent`) :`GameplayEffectClass` "/Game/Blueprints/GameplayEffects/GE_TakeDamage.GE_TakeDamage_C"))

(event `self.HitBox.OnComponentEndOverlap`
  (params (OverlappedComponent :type "PrimitiveComponent Object Reference") (OtherActor :type "Actor Object Reference") (OtherComp :type "PrimitiveComponent Object Reference") (OtherBodyIndex :type Integer))
  ;[1 1 1] For every enemy that leaves range of player, remove one tag of "take damage"
  (cast `/Game/Blueprints/AI/BP_AIPatrolEnemy` OtherActor)
  (`AbilitySystemComponent.RemoveActiveGameplayEffectBySourceEffect` (`self.AbilitySystemComponent`) "/Game/Blueprints/GameplayEffects/GE_TakeDamage.GE_TakeDamage_C" null 1))

(event `OnEnterPortal`
  ;[1 1 1] Entering portal
  (`AbilitySystemComponent.TryActivateAbilitiesByTag` (`self.AbilitySystemComponent`) (`BlueprintGameplayTagLibrary.MakeLiteralGameplayTagContainer` (struct :`GameplayTags` (struct :`(TagName` "Ability.EnterPortal")))) true))

(event `OnShapeshift`
  ;[1 1 1] Handle shapeshifting spell and after 5 seconds return to normal form
  (`self.ChangeVisualToShapeshiftedForm`)
  (`self.PlayerShapeshifted`)
  (`self.DisableInput` null)
  (`KismetSystemLibrary.K2_SetTimerDelegate` (delegate `TransformToNormalForm`) 5.0))

(event `TransformToNormalForm`
  ;[1 1 1] Handle shapeshifting spell and after 5 seconds return to normal form
  (`self.ChangeVisualToNormalForm`)
  (`self.EnableInput` null)
  (`self.PlayerInNormalnForm`))

(event `EnhancedInput|/Game/Input/IA_Shapeshift`
  (params (ActionValue :type Boolean) (ElapsedSeconds :type "Float (double-precision)") (TriggeredSeconds :type "Float (double-precision)") (InputAction :type "InputAction Object Reference" :default "/Game/Input/IA_Shapeshift.IA_Shapeshift"))
  ;[1 1 1] Shapeshift - input key "R"
  (:`Started`
    (`AbilitySystemComponent.TryActivateAbilitiesByTag` (`self.AbilitySystemComponent`) (`BlueprintGameplayTagLibrary.MakeGameplayTagContainerFromTag` (struct :`TagName` "Ability.Shapeshift")) true)))

(event `EnhancedInput|/Game/Input/IA_Jump`
  (params (ActionValue :type Boolean) (ElapsedSeconds :type "Float (double-precision)") (TriggeredSeconds :type "Float (double-precision)") (InputAction :type "InputAction Object Reference" :default "/Game/Input/IA_Jump.IA_Jump"))
  ;[1 1 1] Jump - input key Spacebar
  (:`Started`
    (`AbilitySystemComponent.TryActivateAbilitiesByTag` (`self.AbilitySystemComponent`) (`BlueprintGameplayTagLibrary.MakeGameplayTagContainerFromTag` (struct :`TagName` "Ability.Jump")) true)))

(event `EnhancedInput|/Game/Input/IA_Pause`
  (params (ActionValue :type Boolean) (ElapsedSeconds :type "Float (double-precision)") (TriggeredSeconds :type "Float (double-precision)") (InputAction :type "InputAction Object Reference" :default "/Game/Input/IA_Pause.IA_Pause"))
  (bind _returnvalue (`GameplayStatics.GetPlayerController` 0))
  ;[1 1 1] Open pause menu - input key P
  (:`Started`
    (bind _returnvalue_2 (`|CreateWidget` "/Game/Widgets/WBP_Pause.WBP_Pause_C"))
    (`UserWidget.AddToViewport` _returnvalue_2 0)
    (set `PlayerController.bShowMouseCursor` true _returnvalue)
    (`WidgetBlueprintLibrary.SetInputMode_UIOnlyEx` _returnvalue null)
    (`GameplayStatics.SetGamePaused` true)))

(event `EnhancedInput|/Game/Input/IA_Activate`
  (params (ActionValue :type Boolean) (ElapsedSeconds :type "Float (double-precision)") (TriggeredSeconds :type "Float (double-precision)") (InputAction :type "InputAction Object Reference" :default "/Game/Input/IA_Activate.IA_Activate"))
  (bind _closelever (`self.CloseLever`))
  (bind _closelever_2 (`self.CloseLever`))
  ;[1 1 1] Activate Lever With Key "E"
  (:`Started`
    (`/Engine/EditorBlueprintResources/StandardMacros.IsValid` _closelever_2
      (:`Is Valid`
        (bind _returnvalue (`AbilitySystemComponent.TryActivateAbilitiesByTag` (`self.AbilitySystemComponent`) (`BlueprintGameplayTagLibrary.MakeGameplayTagContainerFromTag` (struct :`TagName` "Ability.Activate")) true)) ; called only to know if player has proper tag = is in range, if yes, we call ability on lever, which is called only if it has not been previously activated
        (if _returnvalue
          (`AbilitySystemComponent.TryActivateAbilitiesByTag` (`AbilitySystemBlueprintLibrary.GetAbilitySystemComponent` _closelever_2) (`BlueprintGameplayTagLibrary.MakeLiteralGameplayTagContainer` (struct :`GameplayTags` (struct :`(TagName` "Ability.LeverActivateItself")))) true)
          (`/Engine/EditorBlueprintResources/StandardMacros.IsValid` _closelever
            (:`Is Valid`
              (`AbilitySystemComponent.BP_ApplyGameplayEffectToTarget` :`self` (`self.AbilitySystemComponent`) :`GameplayEffectClass` "/Game/Blueprints/GameplayEffects/GE_MarkUnableToActivate.GE_MarkUnableToActivate_C" :`Target` (`AbilitySystemBlueprintLibrary.GetAbilitySystemComponent` _closelever)) ; at the end mark lever as already activated so it cannot be activated again
            )))))))

(fn `ChangeVisualToNormalForm`
  (`StaticMeshComponent.SetStaticMesh` (`self.ShapeshiftSM`) null)
  (`SkeletalMeshComponent.SetSkeletalMeshAsset` (`self.Mesh`) "/Game/Animations/Player/SM_PlayerWitch.SM_PlayerWitch")
  (`SkeletalMeshComponent.SetAnimInstanceClass` (`self.Mesh`) "/Game/Animations/Player/ABP_Witch.ABP_Witch_C"))

(fn `ChangeVisualToShapeshiftedForm`
  (`StaticMeshComponent.SetStaticMesh` (`self.ShapeshiftSM`) "/Game/Meshes/tfvnficaa_LOD0.tfvnficaa_LOD0")
  (`SkeletalMeshComponent.SetSkeletalMeshAsset` (`self.Mesh`) null)
  (`SkeletalMeshComponent.SetAnimInstanceClass` (`self.Mesh`) null))

(fn `CheckGrounded`
  ;[1 1 1] Check if player stands on the ground or not
  (if (`NavMovementComponent.IsFalling` (`self.CharacterMovement`))
    (`self.OnFalling`)
    (else
      (`self.OnGrounded`))))

(fn `CheckIfDead`
  ;[1 1 1] Check if health attribute is zero
  (if (<= (`.ReturnValue` (`AbilitySystemComponent.GetGameplayAttributeValue` (`self.AbilitySystemComponent`) (struct :`AttributeName` "Health" :`Attribute` "/Script/AITask.HealthAttributeSet:Health" :`AttributeOwner` "/Script/CoreUObject.Class'\"/Script/AITask.HealthAttributeSet\"'"))) 0.0)
    ;[1 1 1] If yes, apply proper tag and let gamemode know
    (`AbilitySystemComponent.TryActivateAbilitiesByTag` (`self.AbilitySystemComponent`) (`BlueprintGameplayTagLibrary.MakeLiteralGameplayTagContainer` (struct :`GameplayTags` (struct :`(TagName` "Status.Dead")))) true)
    (`/Game/Blueprints/BP_GameMode.PlayerDied` (cast `/Game/Blueprints/BP_GameMode` (`GameplayStatics.GetGameMode`) :!pure true))))

(fn `EraseRefToLever`
  (set `self.CloseLever` null))

(fn `StoreRefToLever`
  (params (LeverRef :type "/Game/Blueprints/BP_Lever Object Reference"))
  (set `self.CloseLever` LeverRef))

(fn `UserConstructionScript`)