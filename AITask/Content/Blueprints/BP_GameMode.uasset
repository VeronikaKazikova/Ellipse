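; Game mode that owns the main HUD widget and handles lever progress, win and loss for the game.
; On begin play it creates the layout UI with game-only input, then relays lever hints and mana bar updates to it.
; Death pauses the game; death and winning both show end screens with a cursor and UI-only input.
; Unlocking the third lever activates the portal actor found in the level.
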(event `self.ReceiveBeginPlay`
  (bind _returnvalue (`GameplayStatics.GetPlayerController` 0))
  ;[0.375 1 0.4466] Begin play: handle UI and cursor
  (set `PlayerController.bShowMouseCursor` false _returnvalue)
  (`WidgetBlueprintLibrary.SetInputMode_GameOnly` _returnvalue)
  (bind _returnvalue_2 (`|CreateWidget` "/Game/Widgets/WBP_Layout.WBP_Layout_C"))
  (bind _output_get (set `self.LayoutUI` _returnvalue_2))
  (`UserWidget.AddToViewport` _output_get 0))

(event `PlayerInLever`
  ;[1 1 1] If player can activate lever, show hint in UI to them, otherwise hide it
  (`/Game/Widgets/WBP_Layout.ShowUnlockHint` (`self.LayoutUI`)))

(event `PlayerLeftLever`
  ;[1 1 1] If player can activate lever, show hint in UI to them, otherwise hide it
  (`/Game/Widgets/WBP_Layout.HideUnlockHint` (`self.LayoutUI`)))

(event `PlayerDied`
  ;[1 1 1] After player death, show proper UI and switch to UI mode
  (`GameplayStatics.SetGamePaused` true)
  (set `PlayerController.bShowMouseCursor` true (cast `Witch_PlayerController` (`GameplayStatics.GetPlayerController` 0) :!pure true))
  (`WidgetBlueprintLibrary.SetInputMode_UIOnlyEx` (`GameplayStatics.GetPlayerController` 0) null)
  (`/Game/Widgets/WBP_Layout.ShowLostScreen` (`self.LayoutUI`)))

(event `WinGame`
  ;[1 1 1] After win, show proper UI and switch to UI mode
  (`/Game/Widgets/WBP_Layout.ShowWinScreen` (`self.LayoutUI`))
  (`WidgetBlueprintLibrary.SetInputMode_UIOnlyEx` (`GameplayStatics.GetPlayerController` 0) null)
  (set `PlayerController.bShowMouseCursor` true (cast `Witch_PlayerController` (`GameplayStatics.GetPlayerController` 0) :!pure true)))

(event `UpdateManaBar`
  ;[1 1 1] Call UI update
  (`/Game/Widgets/WBP_Layout.UpdateManaBar` (`self.LayoutUI`)))

(fn `UnlockAnotherLever`
  (set `self.LeversUnlocked` (+ (`self.LeversUnlocked`) 1))
  (if (== (`self.LeversUnlocked`) 3)
    (bind _returnvalue (`GameplayStatics.GetActorOfClass` "/Game/Blueprints/BP_Portal.BP_Portal_C"))
    (`/Game/Blueprints/BP_Portal.OnActivatePortal` _returnvalue)))

(fn `UserConstructionScript`)